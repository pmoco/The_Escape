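; Player combat component that tracks the current position in an attack combo and resolves which attack comes next.
; AttackList forms a combo graph, where each item holds an attack and a map from trigger enum to the next item's index.
; NextAttack follows a matching trigger and returns the new attack, while ResetCombo returns to the first item, including on BeginPlay.
; ListPossibleAttacks prints an item's available branches for debugging.
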(event `self.ReceiveBeginPlay`
  (`self.ResetCombo`))

(fn `ListPossibleAttacks`
  (params (`combo item` :type "/Game/CombatSystems/Player/ComboItem Structure"))
  (bind _keys (`BlueprintMapLibrary.Map_Keys` `combo item_Triggers_10_4656093349AE633B837C14BDCC695B0C`))
  (for _array_element _keys
    (`KismetSystemLibrary.PrintString` (`KismetStringLibrary.Concat_StrStr` (`|GetEnumeratorNameAsString` _array_element) "- " (`KismetTextLibrary.Conv_TextToString` (break `/Game/CombatSystems/S_Attack` (break `/Game/CombatSystems/Player/ComboItem` (`|GetArrayItem` (`self.AttackList`) (`BlueprintMapLibrary.Map_Find` `combo item_Triggers_10_4656093349AE633B837C14BDCC695B0C` _array_element)))))))))

(fn `NextAttack`
  (params (trigger :type "/Game/ThirdPerson/Blueprints/Actions Enum" :default "NewEnumerator6"))
  (returns (Attack :type "/Game/CombatSystems/S_Attack Structure"))
  (bind (_currentcomboitem_attack _currentcomboitem_triggers) (break `/Game/CombatSystems/Player/ComboItem` (`self.currentComboItem`)))
  (bind (_value _returnvalue) (`BlueprintMapLibrary.Map_Find` _currentcomboitem_triggers trigger))
  (if _returnvalue
    (bind _output_get (set `self.currentComboItem` (`|GetArrayItem` (`self.AttackList`) _value)))
    (return (`.Attack_4_4DC26CD24A517AD735AABDB6FCC762E7` (break `/Game/CombatSystems/Player/ComboItem` _output_get)))))

(fn `ResetCombo`
  (set `self.currentComboItem` (`|GetArrayItem` (`self.AttackList`))))