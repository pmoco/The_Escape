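; Enemy combo component that steps through randomly chosen attack strings, currently only printing attack names rather than executing attacks.
; BeginPlay picks a combo from ComboList, then after a delay starts a self-looping timed event in place of Tick.
; Each cycle advances the combo index, picking a new random combo when the current one runs out, and prints the string with the current attack marked.
; ResetCombo is an empty stub.
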(event `self.ReceiveBeginPlay`
  (`self.PickRandomComboString`)
  (`KismetSystemLibrary.Delay` 5.0)
  (`self.TICK`))

(event `TICK`
  (bind (_currentcombo_attack_element _currentcombo_index) (break `/Game/CombatSystems/Enemy/S_ComboString` (`self.currentCombo`)))
  (`self.NextAttack` :!label _label)
  (`self.ListPossibleAttacks` (`self.currentCombo`) _currentcombo_index)
  (`KismetSystemLibrary.Delay` 2.0)
  (goto _label))

(fn `ListPossibleAttacks`
  (params (`ComboString ` :type "/Game/CombatSystems/Enemy/S_ComboString Structure") (CurrentAttack :type Integer :default -1))
  (locals (text :type String) (AttackName :type Text))
  (for (_array_element _array_index) `ComboString _Attack_element_3_7ED750CA456EA3E463CE60B1FD36854D`
    (set `local.AttackName` (break `/Game/CombatSystems/S_Attack` (break `/Game/CombatSystems/Enemy/S_EnemyAttack` _array_element)))
    (if (== (- CurrentAttack 1) _array_index)
      (set `local.text` (`KismetStringLibrary.Concat_StrStr` (`local.text`) ", -" (`KismetTextLibrary.Conv_TextToString` (`local.AttackName`)) " -"))
      (else
        (set `local.text` (`KismetStringLibrary.Concat_StrStr` (`local.text`) "," (`KismetTextLibrary.Conv_TextToString` (`local.AttackName`)))))))
  (`KismetSystemLibrary.PrintString` (`local.text`)))

(fn `NextAttack`
  (bind (_currentcombo_attack_element _currentcombo_index) (break `/Game/CombatSystems/Enemy/S_ComboString` (`self.currentCombo`)))
  (bind (_currentcombo_attack_element_2 _currentcombo_index_2) (break `/Game/CombatSystems/Enemy/S_ComboString` (`self.currentCombo`)))
  (bind (_currentcombo_attack_element_3 _currentcombo_index_3) (break `/Game/CombatSystems/Enemy/S_ComboString` (`self.currentCombo`)))
  (if (>= _currentcombo_index (`KismetArrayLibrary.Array_Length` _currentcombo_attack_element)) :!label _label
    (`self.PickRandomComboString`)
    (goto _label)
    (else
      (`KismetSystemLibrary.PrintString` (`KismetTextLibrary.Conv_TextToString` (break `/Game/CombatSystems/S_Attack` (break `/Game/CombatSystems/Enemy/S_EnemyAttack` (`|GetArrayItem` _currentcombo_attack_element_2 _currentcombo_index_2)))))
      (`/Engine/EditorBlueprintResources/StandardMacros.IncrementInt` _currentcombo_index_3))))

(fn `PickRandomComboString`
  (bind _output_get (set `self.currentCombo` (`KismetArrayLibrary.Array_Random` (`self.ComboList`))))
  (setmembers `/Game/CombatSystems/Enemy/S_ComboString` :`StructRef` _output_get :`index` 0))

(fn `ResetCombo`)