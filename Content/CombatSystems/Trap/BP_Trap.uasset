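; BP_Trap is a spike trap that cycles up and down and damages actors that overlap it.
; Five seconds after BeginPlay, an endless delay loop flips Active and slides the Trap component between its raised and base positions with MoveComponentTo.
; Overlapping actors receive Damage through BPI_Damegeable regardless of Active, with a debug print on success.
; Attack, GetAttackName, GetCanAttack and HitDetection are stubs returning empty or false values.
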(event `self.ReceiveBeginPlay`
  (`self.TriggerTrap`))

(event `TriggerTrap`
  (bind _active (`self.active`))
  (bind _trap (`self.Trap`))
  (bind _trap_2 (`self.Trap`))
  (bind (_returnvalue_location _returnvalue_rotation) (`KismetMathLibrary.BreakTransform` (`SceneComponent.GetRelativeTransform` _trap_2)))
  (bind (_returnvalue_location_2 _returnvalue_rotation_2) (`KismetMathLibrary.BreakTransform` (`SceneComponent.GetRelativeTransform` _trap)))
  (`KismetSystemLibrary.Delay` 5.0)
  (`KismetSystemLibrary.PrintString` (`KismetStringLibrary.Conv_BoolToString` _active))
  (if _active :!label _label
    (`KismetSystemLibrary.MoveComponentTo` _trap_2 (0.0 0.0 0.0) _returnvalue_rotation false false 1.0)
    (else
      (`KismetSystemLibrary.MoveComponentTo` _trap (0.0 0.0 50.0) _returnvalue_rotation_2 false false 1.0)))
  (set `self.active` (not (`self.active`)))
  (`KismetSystemLibrary.Delay` 3.0)
  (goto _label))

(event `self.ReceiveActorBeginOverlap`
  (params (OtherActor :type "Actor Object Reference"))
  (bind _asbpi_damegeable (cast `/Game/CombatSystems/BPI_Damegeable` OtherActor))
  (bind _wasdamaged (`/Game/CombatSystems/BPI_Damegeable.TakeDamage` _asbpi_damegeable (`self.Damage`)))
  (if _wasdamaged
    (`KismetSystemLibrary.PrintString` "HEHEHE SPIKES!" true true (struct :`R` 1.0 :`G` 0.954361 :`B` 0.934119 :`A` 1.0))))

(fn `Attack`
  (params (Attack :type "/Game/CombatSystems/S_Attack Structure"))
  (returns (AttackHit :type Boolean) (wasBlocked :type Boolean) (wasParried :type Boolean))
  (return false false false))

(fn `getAttackName`
  (returns (Name :type Text))
  (return ""))

(fn `getCanAttack`
  (returns (canAttack :type Boolean))
  (return false))

(fn `HitDetection`
  (returns (hit :type Boolean) (hitResult :type "HitResult Structure"))
  (return false))

(fn `UserConstructionScript`)