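; Actor component that owns a character's health, handling healing, incoming damage and death for combat.
; TakeDamage passes a damage struct through the CanBeDamaged macro, which routes to block, damage or no damage based on dead, invincible and blocking state.
; Results fire OnBlock, OnDeath, or OnTakeDamage with a damage response when the hit can or must interrupt.
; Heal adds health clamped to MaxHealth while alive.
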(fn `Heal`
  (params (Amount :type "Float (double-precision)"))
  (returns (`New Health` :type "Float (double-precision)"))
  (if (not (`self.isDead`))
    (set `self.Health` (`KismetMathLibrary.FClamp` (+ Amount (`self.Health`)) 0.0 (`self.MaxHealth`)))
    (return 0.0)))

(fn `TakeDamage`
  (params (Damage :type "/Game/CombatSystems/S_DamageInfo Structure"))
  (returns (WasDamaged :type Boolean))
  (bind (_amount _damagetype _damageresponse _shoulddamageinvicible _canbeblocked _canbeparried _shouldforceinterrupt) (break `/Game/CombatSystems/S_DamageInfo` Damage))
  (`self.CanBeDamaged` _shoulddamageinvicible _canbeblocked
    (:`BlockDamage`
      (`self.onBlock` _canbeparried)
      (return false))
    (:`DoDamage`
      (bind _output_get (set `self.Health` (- (`self.Health`) _amount)))
      (if (<= _output_get 0.0)
        (set `self.isDead` true)
        (`self.onDeath`)
        (return true)
        (elif (or (`self.isInterruptable`) _shouldforceinterrupt)
          (`self.onTakeDamage` _damageresponse)
          (return true))))
    (:`NoDamage`
      (return false))))