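; Actor component that provides blocking for a Character owner in the combat system.
; Block plays the block montage on the owner, fires the StartBlocking dispatcher and prints the montage name for debugging.
; BlockDetection and StopBlock set and clear the IsBlocking flag separately from Block, with no damage handling in the component itself.
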(fn `Block`
  (bind _blockanimation (`self.BlockAnimation`))
  (bind _ascharacter (cast `Character` (`self.GetOwner`)))
  (`Character.PlayAnimMontage` _ascharacter _blockanimation 1.0 "None")
  (`self.StartBlocking `)
  (`KismetSystemLibrary.PrintString` (`KismetSystemLibrary.GetDisplayName` _blockanimation)))

(fn `BlockDetection`
  (set `self.isBlocking ` true))

(fn `StopBlock`
  (set `self.isBlocking ` false))