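; Combat component that runs a character's attacks, from montage playback to weapon hit detection and damage.
; Attack, gated by CanAttack, stores the attack struct, sets the Attacking state, fires OnAttack and plays the montage; ResetAttack clears them.
; HitDetection sphere-traces between weapon sockets with debug drawing, skipping actors already in Hits.
; BPI_Damegeable targets receive damage; OnHit flags undamaged or non-damageable hits as blocked, and empty traces fire OnMiss.
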(fn `Attack `
  (params (Attack :type "/Game/CombatSystems/S_Attack Structure"))
  (returns (canAttack :type Boolean))
  (if (`self.canAttack`)
    (bind _output_get (set `self.Attack` Attack))
    (set `self.state ` "Attacking")
    (bind (_name _animation) (break `/Game/CombatSystems/S_Attack` _output_get))
    (`self.OnAttack` _animation)
    (`KismetSystemLibrary.PrintString` (`KismetTextLibrary.Conv_TextToString` _name))
    (bind _ascharacter (cast `Character` (`self.GetOwner`)))
    (`Character.PlayAnimMontage` _ascharacter (`.Animation_14_40C66D98460438FDF39437B1B4F9B947` (break `/Game/CombatSystems/S_Attack` (`self.Attack`))) 1.0 "None")
    (return true)))

(fn `getAttackName`
  (returns (NewParam :type Text))
  (return (`.Name_2_58D90697411CFBE7A2100D8BEEA9627E` (break `/Game/CombatSystems/S_Attack` (`self.Attack`)))))

(fn `hitDetection`
  (params (WeaponSocketStart :type "Vector Structure") (WeaponSocketEnd :type "Vector Structure"))
  (returns (wasHit :type Boolean) (wasDamage :type Boolean))
  (locals (hits :type "Array of Actor Object Reference") (`Damaged?` :type Boolean :default false))
  (bind (_attack_name _attack_animation _attack_damage) (break `/Game/CombatSystems/S_Attack` (`self.Attack`)))
  (bind _hits (`local.hits`))
  (set `local.Damaged?` false)
  (bind (_outhits _returnvalue) (`KismetSystemLibrary.SphereTraceMultiForObjects` :`Start` WeaponSocketStart :`End` WeaponSocketEnd :`Radius` 5.0 :`ObjectTypes` (`|MakeArray` "ObjectTypeQuery3" "ObjectTypeQuery4" "ObjectTypeQuery1" "ObjectTypeQuery2" "ObjectTypeQuery6" :!type "EObjectTypeQuery Enum") :`DrawDebugType` "ForDuration" :`DrawTime` 2.0))
  (for _array_element _outhits
    (bind (_bblockinghit _binitialoverlap _time _distance _location _impactpoint _normal _impactnormal _physmat _hitactor) (`GameplayStatics.BreakHitResult` _array_element))
    (if (not (`KismetArrayLibrary.Array_Contains` _hits _hitactor))
      (`KismetArrayLibrary.Array_AddUnique` _hits _hitactor)
      (`self.processHit` _hitactor
        (:`RandomMesh`
          (`self.OnHit` _attack_animation true))
        (:`Damageable`
          (bind _wasdamaged (message `/Game/CombatSystems/BPI_Damegeable.TakeDamage` _hitactor _attack_damage))
          (bind _output_get (set `local.Damaged?` _wasdamaged))
          (bind _returnvalue_2 (not _output_get))
          (`KismetSystemLibrary.PrintString` (`KismetStringLibrary.Concat_StrStr` "ASASASAS" (`KismetStringLibrary.Conv_BoolToString` _returnvalue_2)) true true (struct :`R` 1.0 :`G` 0.093193 :`A` 1.0))
          (`self.OnHit` _attack_animation _returnvalue_2)))))
  (if (not _returnvalue)
    (`self.OnMiss`)
    (return _returnvalue (`local.Damaged?`))))

(fn `resetAttack `
  (set `self.canAttack` true)
  (set `self.state ` "")
  (set `self.Attack` (make `/Game/CombatSystems/S_Attack` "" null)))